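; Pong ball actor that moves on the XZ plane and bounces off the paddles and walls.
; BeginPlay caches the PongGameMode and calls Reset, which centers the ball, restores base speed and picks a random diagonal direction.
; Tick moves it by lerping with delta time as alpha, without sweeping.
; Overlaps drive bounces: paddles flip X and add speed, while top and bottom walls flip Z.
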(event EventBeginPlay
  (Utilities|FlowControl|Sequence
    (:then_0
      (bind _aspong_game_mode (Utilities|Casting|CastToPongGameMode (Game|GetGameMode)))
      (Variables|Default|SetGameMode _aspong_game_mode))
    (:then_1
      (CallFunction|Reset))))

(event EventTick
  (params (DeltaSeconds :type Float%20%28single-precision%29))
  (CallFunction|Update DeltaSeconds))

(event Collision|EventActorBeginOverlap
  (params (OtherActor :type Actor%20Object%20Reference))
  (CallFunction|Collide OtherActor))

(fn ConstructionScript)

(fn Reset
  (Transformation|SetActorLocation "0, 0, 0" false false) ; Move to starting position in the middle of the screen.
  (Variables|Default|SetVelocity 2.5e+02) ; Stop the movement.
  (Variables|Default|SetDirection (Math|Vector|Normalize (Utilities|Select :Index (Math|Random|RandomInteger 4) :Option%200 "1.000000, 0,1.000000" :Option%201 "1.000000,0.000000,-1.000000" :Option%202 "-1.000000,0.000000,1.000000" :Option%203 "-1.000000,0.000000,-1.000000"))) ; Randomize a new direction.
)

(fn Update
  (params (Delta :type Float%20%28single-precision%29))
  (bind _returnvalue (Transformation|GetActorLocation))
  (Transformation|SetActorLocation (Math|Vector|Lerp(Vector) _returnvalue (+ _returnvalue (* (Variables|Default|GetDirection) (Variables|Default|GetVelocity))) Delta) false false))

(fn Collide
  (params (Actor :type Actor%20Object%20Reference))
  (if (or (== Actor (Variables|Default|GetLeftPaddle)) (== Actor (Variables|Default|GetRightPaddle)))
    (Variables|Default|SetDirection (Utilities|InverseVectorX (Variables|Default|GetDirection)))
    (Variables|Default|SetVelocity (+ (Variables|Default|GetVelocity) 5e+01)) ; Increment velocity.
    (elif (or (== Actor (Variables|Default|GetTopWall)) (== Actor (Variables|Default|GetBottomWall)))
      (Variables|Default|SetDirection (Utilities|InverseVectorZ (Variables|Default|GetDirection))))))