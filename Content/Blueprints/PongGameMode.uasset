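; Game mode for a Pong game that tracks both players' scores and ends the match when one wins.
; Separate events increment the left and right player scores and compare the result with ScoreTarget.
; Both win checks feed a shared path that waits briefly, then opens the MainMenu level.
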(event Custom|IncrementLeftPlayerScore
  (bind _result (Math|Integer|IncrementInt (Variables|Default|GetLeftPlayerScore))
    (:%20%20
      (if (>= _result (Variables|Default|GetScoreTarget)) ; We have a winner?
        (Utilities|FlowControl|Delay 1.0)
        (Game|OpenLevel(byName) "MainMenu")))))

(event Custom|IncrementRightPlayerScore
  (bind _result (Math|Integer|IncrementInt (Variables|Default|GetRightPlayerScore))
    (:%20%20
      (if (>= _result (Variables|Default|GetScoreTarget)) ; We have a winner?
        (Utilities|FlowControl|Delay 1.0)
        (Game|OpenLevel(byName) "MainMenu")))))

(fn ConstructionScript)